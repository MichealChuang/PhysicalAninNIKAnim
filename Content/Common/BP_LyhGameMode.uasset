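; Game mode Blueprint that handles respawning a player through its Reborn event.
; Reborn spawns a new BP_LyhActDemoCharacter using the X and Y of randomly picked TargetPoint actors in the level, at a fixed height.
; The given controller possesses the new character and switches to game-only input, then the old pawn is destroyed.
; If the controller is a PC_lyh, its HUD is initialized again through InitialHUD.
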(event `Reborn`
  (params (Controller :type "PlayerController Object Reference"))
  (set `self.OriginPawn` (`Controller.K2_GetPawn` Controller))
  (bind _outactors (`GameplayStatics.GetAllActorsOfClass` "/Script/Engine.TargetPoint"))
  (bind (_returnvalue_x _returnvalue_y) (`KismetMathLibrary.BreakVector` (`self.K2_GetActorLocation` (`|GetArrayItem` _outactors (`KismetMathLibrary.RandomIntegerInRange` 0 (`KismetArrayLibrary.Array_LastIndex` _outactors))))))
  (bind _returnvalue (`|SpawnActorFromClass` "/Game/Common/BP_LyhActDemoCharacter.BP_LyhActDemoCharacter_C" (`KismetMathLibrary.MakeTransform` (`KismetMathLibrary.MakeVector` _returnvalue_x _returnvalue_y 228.0)) "Undefined" "OverrideRootScale" null null))
  (`Controller.Possess` Controller _returnvalue)
  (`WidgetBlueprintLibrary.SetInputMode_GameOnly` Controller)
  (`self.K2_DestroyActor` (`self.OriginPawn`))
  (bind _aspc_lyh (cast `/Game/Common/PC_lyh` Controller))
  (`/Game/Common/PC_lyh.InitialHUD` _aspc_lyh))

(fn `UserConstructionScript`)