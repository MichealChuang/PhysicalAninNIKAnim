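; Player demo character that greets or challenges AI characters and carries a child-actor sword on its hand socket.
; Tick feeds its location to the Col_OutLine parameter collection, while Y plays or reverses a timeline driving that effect's radius.
; G resets combat flags and toggles the WBP_Hello widget with matching input mode.
; Hello and Fight find an AI via CheckAI and notify it after a montage; Defeated and Victory handle outcome montages, UI and input.
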(event `self.ReceiveTick`
  (params (DeltaSeconds :type "Float (single-precision)"))
  (`KismetMaterialLibrary.SetVectorParameterValue` "/Game/Material/Col_OutLine.Col_OutLine" "Location" (`KismetMathLibrary.Conv_VectorToLinearColor` (`self.K2_GetActorLocation`))))

(event `Key|Y`
  (params (Key :type "Key Structure"))
  (:`Pressed`
    (`/Engine/EditorBlueprintResources/StandardMacros.FlipFlop`
      (:`A`
        (bind (_direction _newtrack_0) (`Timeline|Timeline_0` :!via `PlayFromStart` :!label _label)
          (:`Update`
            (`KismetMaterialLibrary.SetScalarParameterValue` "/Game/Material/Col_OutLine.Col_OutLine" "Radius" _newtrack_0))))
      (:`B`
        (goto _label :!via `Reverse`)))))

(event `initialState`
  (set `self.bCanDamage` false)
  (set `self.bIsAttacking` false)
  (set `self.bIsDodging` false)
  (set `self.bIsDefencing` false))

(event `Key|G`
  (params (Key :type "Key Structure"))
  (bind _returnvalue (`GameplayStatics.GetPlayerController` 0))
  (bind _widgetref (`self.WidgetRef`))
  (:`Pressed`
    (`self.initialState`)
    (`/Engine/EditorBlueprintResources/StandardMacros.FlipFlop`
      (:`A`
        (`/Engine/EditorBlueprintResources/StandardMacros.IsValid` (`self.WidgetRef`)
          (:`Is Valid`
            _)
          (:`Is Not Valid`
            (bind _returnvalue_2 (`|CreateWidget` "/Game/UI/WBP_Hello.WBP_Hello_C" (`GameplayStatics.GetPlayerController` 0)))
            (set `self.WidgetRef` _returnvalue_2)))
        (`UserWidget.AddToViewport` _widgetref 0)
        (set `PlayerController.bShowMouseCursor` true _returnvalue)
        (`WidgetBlueprintLibrary.SetInputMode_GameAndUIEx` _returnvalue (`self.WidgetRef`)))
      (:`B`
        (`Widget.RemoveFromParent` _widgetref)
        (set `PlayerController.bShowMouseCursor` false _returnvalue)
        (`WidgetBlueprintLibrary.SetInputMode_GameOnly` _returnvalue)))))

(event `Hello`
  (bind _returnvalue (`self.CheckAI` 90.0 1000.0 (`|MakeArray` "ObjectTypeQuery3" :!type "EObjectTypeQuery Enum") false (`|MakeArray` null :!type "Actor Object Reference") "Persistent" true (struct :`R` 1.0 :`A` 1.0) (struct :`G` 1.0 :`A` 1.0) 5.0))
  (`/Engine/EditorBlueprintResources/StandardMacros.IsValid` _returnvalue
    (:`Is Valid`
      (`KismetSystemLibrary.PrintString` "hhhhhhhhhhhhhhhhhhhello"))
    (:`Is Not Valid`
      (`KismetSystemLibrary.PrintString` "bbbbbbbbbbbbbbbbbbbye")))
  (bind _returnvalue_2 (`self.PlayAnimMontage` "/Game/Animations/AnimMontage/Hello.Hello"))
  (bind _asbp_aicharacter (cast `/Game/AI/BP_AICharacter` _returnvalue))
  (`KismetSystemLibrary.Delay` _returnvalue_2)
  (`/Game/AI/BP_AICharacter.Hello` _asbp_aicharacter (`self.K2_GetActorLocation`)))

(event `Fight`
  (bind _returnvalue (`self.CheckAI` 30.0 1000.0 (`|MakeArray` "ObjectTypeQuery3" :!type "EObjectTypeQuery Enum") false (`|MakeArray` self :!type "Actor Object Reference") "None" true (struct :`R` 1.0 :`A` 1.0) (struct :`G` 1.0 :`A` 1.0) 5.0))
  (bind _returnvalue_2 (`self.PlayAnimMontage` "/Game/Animations/AnimMontage/FightRequest.FightRequest"))
  (bind _asbp_aicharacter (cast `/Game/AI/BP_AICharacter` _returnvalue))
  (`KismetSystemLibrary.Delay` _returnvalue_2)
  (`self.PlayAnimMontage` "/Game/Animations/AnimMontage/Ready.Ready")
  (`/Game/AI/BP_AICharacter.Fight` _asbp_aicharacter self))

(event `self.Defeated`
  (bind _returnvalue (`GameplayStatics.GetPlayerController` 0))
  (`self.PlayAnimMontage` "/Game/Animations/AnimMontage/Surrender.Surrender")
  (bind _returnvalue_2 (`|CreateWidget` "/Game/UI/WBP_Death.WBP_Death_C" _returnvalue))
  (`UserWidget.AddToViewport` _returnvalue_2 0)
  (`WidgetBlueprintLibrary.SetInputMode_UIOnlyEx` _returnvalue _returnvalue_2)
  (set `PlayerController.bShowMouseCursor` true _returnvalue))

(event `Victory`
  (bind _returnvalue (`GameplayStatics.GetPlayerController` 0))
  (`self.initialState`)
  (`self.DisableInput` _returnvalue)
  (bind _returnvalue_2 (`self.PlayAnimMontage` "/Game/Animations/AnimMontage/Victory.Victory"))
  (`KismetSystemLibrary.Delay` _returnvalue_2)
  (`self.EnableInput` _returnvalue))

(event `self.InitialSwordState`
  (bind _asbp_sword (cast `/Game/Common/BP_Sword` (`ChildActorComponent.ChildActor` (`self.ChildActor`))))
  (set `Sword.bHasSucceed` false _asbp_sword))

(fn `UserConstructionScript`
  (`SceneComponent.K2_AttachToComponent` (`self.ChildActor`) (`self.Mesh`) "hand_rSocket" "SnapToTarget" "SnapToTarget" "KeepRelative" true))