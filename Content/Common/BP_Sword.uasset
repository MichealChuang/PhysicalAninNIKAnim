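; BP_Sword is a melee weapon, owned by its HumanLike parent actor, that resolves hits on overlap while the owner can damage.
; Dodges and blocks negate hits; for AI attackers they reset blackboard state, and blocks rebound OnAttacked onto the attacker.
; Confirmed hits damage and play sound, with timeline-weighted partial ragdoll and impulse on non-pelvis bones.
; Outcomes update player-controller AI info, victory, or the AI attacker's blackboard.
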(event `self.InitialOwner`
  (bind _ashuman_like (cast `HumanLike` (`self.GetParentActor`)))
  (set `self.OwnerRef` _ashuman_like))

(event `self.ReceiveTick`
  (params (DeltaSeconds :type "Float (single-precision)"))
  (bind _bonename (`self.BoneName`))
  (bind _mesh (`Character.Mesh` (`self.EnemyRef`)))
  (if (> (`self.Weight`) 0.0)
    (`SkeletalMeshComponent.SetAllBodiesBelowSimulatePhysics` _mesh _bonename true true)
    (`SkeletalMeshComponent.SetAllBodiesBelowPhysicsBlendWeight` _mesh _bonename (`self.Weight`) false true)))

(event `self.Collision.OnComponentBeginOverlap`
  (params (OverlappedComponent :type "PrimitiveComponent Object Reference") (OtherActor :type "Actor Object Reference") (OtherComp :type "PrimitiveComponent Object Reference") (OtherBodyIndex :type Integer) (bFromSweep :type Boolean) (SweepResult :type "HitResult Structure (by ref)"))
  (bind _battackedsucceed (`self.bAttackedSucceed`))
  (bind _ownerref (`self.OwnerRef`))
  (bind _enemyref (`self.EnemyRef`))
  (bind _stats_blood (break `PlayerStats` (`HumanLike.Stats` _enemyref)))
  (bind _mesh (`Character.Mesh` (`self.EnemyRef`)))
  (bind _blackboardref (`/Game/AI/PC_AI.BlackBoardRef` (cast `/Game/AI/PC_AI` (`Pawn.GetController` (`self.OwnerRef`)) :!pure true)))
  (if (not (`self.bHasSucceed`))
    (`/Engine/EditorBlueprintResources/StandardMacros.IsValid` _ownerref
      (:`Is Valid`
        (if (`LyhActDemoCharacter.bCanDamage` _ownerref)
          (bind _ashuman_like (cast `HumanLike` OtherActor))
          (if (!= _ashuman_like (`self.OwnerRef`))
            (bind _output_get (set `self.EnemyRef` _ashuman_like))
            (if (or (`LyhActDemoCharacter.bIsDodging` _output_get) (`LyhActDemoCharacter.bIsDefencing` _output_get))
              (bind _aspc_ai (cast `/Game/AI/PC_AI` (`Pawn.GetController` (`self.OwnerRef`))))
              (bind _blackboardref_2 (`/Game/AI/PC_AI.BlackBoardRef` _aspc_ai))
              (`BlackboardComponent.ClearValue` _blackboardref_2 (`self.EnemyTarget`))
              (`BlackboardComponent.SetValueAsBool` _blackboardref_2 (`self.bAttackedSucceed`) false)
              (if (`HumanLike.bIsDefencing` (`self.EnemyRef`))
                (`HumanLike.OnAttacked` (`self.OwnerRef`) (0.0 0.0 0.0)))
              (else
                (bind _returnvalue (`self.CheckHitLocation` (`|MakeArray` "ObjectTypeQuery4" "ObjectTypeQuery3" :!type "EObjectTypeQuery Enum") (`self.OwnerRef`) (`self.EnemyRef`) "ForDuration"))
                (if (`self.bHasSucceed`)
                  (`AICharacter.OnAttacked` (`self.EnemyRef`) _returnvalue)
                  (`GameplayStatics.PlaySoundAtLocation` "/Game/Sounds/Sword_Stab_Cue.Sword_Stab_Cue" _returnvalue)
                  (`|ExecutionSequence`
                    (:`then_0`
                      (if (!= (`self.BoneName`) "pelvis")
                        (`|ExecutionSequence`
                          (:`then_0`
                            (bind (_direction _weight) (`Timeline|Timeline_1` :!via `PlayFromStart`)
                              (:`Update`
                                (set `self.Weight` _weight))
                              (:`Finished`
                                (`SkeletalMeshComponent.SetAllBodiesPhysicsBlendWeight` _mesh 0.0 false)
                                (`SkeletalMeshComponent.SetAllBodiesSimulatePhysics` _mesh false))))
                          (:`then_1`
                            (`KismetSystemLibrary.Delay` 0.1)
                            (`PrimitiveComponent.AddImpulse` _mesh (* (`KismetMathLibrary.GetForwardVector` (`self.K2_GetActorRotation` (`self.OwnerRef`))) 1200.0) (`self.BoneName`) true)))))
                    (:`then_1`
                      (bind _asbp_aicharacter (cast `/Game/AI/BP_AICharacter` _enemyref)
                        (:`then`
                          (bind _aspc_lyh (cast `/Game/Common/PC_lyh` (`GameplayStatics.GetPlayerController` 0)))
                          (`/Game/Common/PC_lyh.InitialAI` _aspc_lyh _asbp_aicharacter)
                          (if (<= _stats_blood 0)
                            (`/Game/Common/BP_LyhActDemoCharacter.Victory` (cast `/Game/Common/BP_LyhActDemoCharacter` (`self.OwnerRef`) :!pure true))))
                        (:`CastFailed`
                          (bind _asbp_lyh_act_demo_character (cast `/Game/Common/BP_LyhActDemoCharacter` _enemyref))
                          (bind _stats_blood_2 (break `PlayerStats` (`HumanLike.Stats` _asbp_lyh_act_demo_character)))
                          (if (<= _stats_blood_2 0)
                            (`BlackboardComponent.ClearValue` _blackboardref (`self.EnemyTarget`))
                            (`BlackboardComponent.SetValueAsBool` _blackboardref _battackedsucceed false)
                            (`/Game/AI/BP_AICharacter.ClearFace` (cast `/Game/AI/BP_AICharacter` (`self.OwnerRef`) :!pure true))
                            (else
                              (`BlackboardComponent.SetValueAsBool` _blackboardref _battackedsucceed true))))))))))))))))

(fn `UserConstructionScript`)