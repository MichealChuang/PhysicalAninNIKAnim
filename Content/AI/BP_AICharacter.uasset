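; AI character with a sword child actor on its right hand that can greet, fight and surrender to the player.
; Hello and Fight turn it toward the player and play montages; Fight also sets the blackboard EnemyTarget and starts a looping timer that keeps it facing player 0.
; Defeated resets combat flags, clears target and timer, then resets the first Stats field after the Surrender montage.
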(event `initialState`
  (set `self.bCanDamage` false)
  (set `self.bIsAttacking` false))

(event `Hello`
  (params (PlayerLocation :type "Vector Structure"))
  (`self.K2_SetActorRotation` (`KismetMathLibrary.FindLookAtRotation` (`self.K2_GetActorLocation`) PlayerLocation))
  (`self.PlayAnimMontage` "/Game/Animations/AnimMontage/AI_What.AI_What"))

(event `Fight`
  (params (Player :type "/Game/Common/BP_LyhActDemoCharacter Object Reference"))
  (`/Engine/EditorBlueprintResources/StandardMacros.IsValid` Player
    (:`Is Valid`
      (`self.K2_SetActorRotation` (`KismetMathLibrary.FindLookAtRotation` (`self.K2_GetActorLocation`) (`self.K2_GetActorLocation` Player)))
      (`self.PlayAnimMontage` "/Game/Animations/AnimMontage/Ready.Ready")
      (bind _aspc_ai (cast `/Game/AI/PC_AI` (`AIBlueprintHelperLibrary.GetAIController` self))
        (:`then`
          (bind _output_get (set `self.BlackBoard` (`/Game/AI/PC_AI.BlackBoardRef` _aspc_ai)))
          (`BlackboardComponent.SetValueAsObject` _output_get (`self.EnemyTarget`) Player)
          (bind _returnvalue (`KismetSystemLibrary.K2_SetTimerDelegate` (delegate `RotateSelf`) 0.5 true))
          (set `self.FaceHandle` _returnvalue))
        (:`CastFailed`
          (`KismetSystemLibrary.PrintString` "PC_AI Cast failed"))))
    (:`Is Not Valid`
      (`KismetSystemLibrary.PrintString` "Player Not Valid"))))

(event `RotateSelf`
  (bind (_returnvalue_roll _returnvalue_pitch _returnvalue_yaw) (`KismetMathLibrary.BreakRotator` (`KismetMathLibrary.FindLookAtRotation` (`self.K2_GetActorLocation`) (`self.K2_GetActorLocation` (`GameplayStatics.GetPlayerCharacter` 0)))))
  (`self.K2_SetActorRotation` (`KismetMathLibrary.MakeRotator` 0.0 0.0 _returnvalue_yaw)))

(event `ClearFace`
  (`KismetSystemLibrary.K2_ClearAndInvalidateTimerHandle` (`self.FaceHandle`)))

(event `self.Defeated`
  (bind _blackboard (`self.BlackBoard`))
  (bind (_stats_blood _stats_magic _stats_magicregain) (break `PlayerStats` (`self.Stats`)))
  (`self.initialState`)
  (`/Engine/EditorBlueprintResources/StandardMacros.IsValid` _blackboard
    (:`Is Valid`
      (`BlackboardComponent.ClearValue` _blackboard (`self.EnemyTarget`))
      (`self.ClearFace`))
    (:`Is Not Valid`
      _))
  (bind _returnvalue (`self.PlayAnimMontage` "/Game/Animations/AnimMontage/Surrender.Surrender"))
  (`KismetSystemLibrary.Delay` _returnvalue)
  (set `self.Stats` (make `PlayerStats` 200 _stats_magic _stats_magicregain)))

(event `self.InitialSwordState`
  (bind _asbp_sword (cast `/Game/Common/BP_Sword` (`ChildActorComponent.ChildActor` (`self.ChildActor`))))
  (set `Sword.bHasSucceed` false _asbp_sword))

(fn `UserConstructionScript`
  (`SceneComponent.K2_AttachToComponent` (`self.ChildActor`) (`self.Mesh`) "hand_rSocket" "SnapToTarget" "SnapToTarget" "KeepRelative" true))